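; Test Dream Eater is a sword-and-shield melee NPC that fights the ThirdPersonCharacter.
; Draw and sheathe montages gate attacking and re-socket the sword; drawing also starts a recursive random block loop.
; Attacks chain into a three-montage combo via buffered input, and box overlaps deal damage while the hit flag is set.
; Blocks succeed only against roughly opposing yaw and notify the attacker; getting blocked briefly stuns this NPC.
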(event `self.ReceiveBeginPlay`
  ;[1 1 1] Attach Wep to NPC
  (`SceneComponent.K2_AttachToComponent` (`self.Sword`) (`self.Mesh`) "weapon_back" "SnapToTarget" "SnapToTarget" "KeepRelative" true)
  (`SceneComponent.K2_AttachToComponent` (`self.shield`) (`self.Mesh`) "hand_l" "KeepWorld" "KeepWorld" "KeepWorld" true))

(event `RandomBlock`
  ;[1 1 1] If AI stood still & Not Stunned, Block
  ;
  ; If AI Moving OR Stunned, Don't Block
  (if (not (or (> (`KismetMathLibrary.VSize` (`MovementComponent.Velocity` (`self.CharacterMovement`))) 100.0) (`self.Stunned`)))
    ;[1 1 1] Block
    (set `self.Block` true))
  ;[1 1 1] Generate A Random Number
  (if (== (`KismetMathLibrary.RandomIntegerInRange` 0 3) 0)
    ;[1 1 1] If Random Number = 0, Stop Blocking for 2 seconds, Send Event Again
    (set `self.Block` false)
    (`KismetSystemLibrary.Delay` 2.0)
    (else
      ;[1 1 1] If Random Number = 1,2,3 Keep Blocking, Send Event Again
      (`KismetSystemLibrary.Delay` 1.0)))
  (`self.RandomBlock`))

(event `Attack Player`
  ;[1 1 1] Attacking + Combos
  (if (`self.ReadyToAttack?`)
    (if (`self.Stunned`)
      _
      (elif (`self.Attacking?`)
        (set `self.SaveAttack` true)
        (else
          (set `self.Attacking?` true)
          (set `self.Block` false)
          (switch `int` (`self.AttackCount`) :!label _label
            (:`0`
              (set `self.AttackCount` 1)
              (`self.PlayAnimMontage` "/Game/Mannequin/Animations/Attack_A_Montage.Attack_A_Montage"))
            (:`1`
              (set `self.AttackCount` 2)
              (`self.PlayAnimMontage` "/Game/Mannequin/Animations/Attack_B_Montage.Attack_B_Montage"))
            (:`2`
              (set `self.AttackCount` 3)
              (`self.PlayAnimMontage` "/Game/Mannequin/Animations/Attack_C_Montage.Attack_C_Montage"))))))))

(event `AttackCombo`
  ;[1 1 1] Attacking + Combos
  (if (`self.SaveAttack`)
    (set `self.SaveAttack` false)
    (if (== (`self.AttackCount`) 3)
      (`KismetSystemLibrary.Delay` 0.7)
      (else
        (goto _label))))
  (set `self.AttackCount` 0)
  (set `self.Attacking?` false))

(event `DrawWeapon`
  ;[1 1 1] Draw Weapon/Character Attack
  (if (not (`self.WeaponDrawn?`))
    (`/Engine/EditorBlueprintResources/StandardMacros.DoOnce` false :!label _label_2
      (:`Completed`
        (bind _returnvalue (`self.PlayAnimMontage` "/Game/Mannequin/Animations/DrawSwordAnim.DrawSwordAnim"))
        (`KismetSystemLibrary.Delay` _returnvalue)
        (set `self.ReadyToAttack?` true)
        (`self.RandomBlock`)
        (goto _label_2 :!via `Reset`)))))

(event `SheatheWeapon`
  ;[1 1 1] Sheathe Weapon
  (if (`self.WeaponDrawn?`)
    (`/Engine/EditorBlueprintResources/StandardMacros.DoOnce` false :!label _label_3
      (:`Completed`
        (set `self.ReadyToAttack?` false)
        (bind _returnvalue (`self.PlayAnimMontage` "/Game/Mannequin/Animations/SheatheSwordAnim.SheatheSwordAnim"))
        (`KismetSystemLibrary.Delay` _returnvalue)
        (goto _label_3 :!via `Reset`)))))

(event `DrawSword`
  ;[1 1 1] Attach Weapon To Character
  (`SceneComponent.K2_AttachToComponent` (`self.Sword`) (`self.Mesh`) "hand_r" "KeepWorld" "KeepWorld" "KeepWorld" true)
  (set `self.WeaponDrawn?` true))

(event `SheatheSword`
  ;[1 1 1] Attach Weapon To Character
  (`SceneComponent.K2_AttachToComponent` (`self.Sword`) (`self.Mesh`) "weapon_back" "KeepWorld" "KeepWorld" "KeepWorld" true)
  (set `self.WeaponDrawn?` false))

(event `self.ReceiveAnyDamage`
  (params (Damage :type "Float (single-precision)") (DamageType :type "DamageType Object Reference") (InstigatedBy :type "Controller Object Reference") (DamageCauser :type "Actor Object Reference"))
  ;[1 1 1] Take Damage
  (set `self.AttackingActor` DamageCauser)
  (if (`self.Block`)
    (bind _faceinai (`self.BlockAngleCheck`))
    (if _faceinai
      (`KismetSystemLibrary.PrintString` "block")
      (message `/Game/AI_DIOPORCO/AttackBlockBP.Attack Blocked` DamageCauser)
      (else
        (bind _output_get (set `self.Health` (- (`self.Health`) Damage) :!label _label_4))
        (`KismetSystemLibrary.PrintString` (`KismetStringLibrary.Conv_DoubleToString` _output_get))
        (`self.PlayAnimMontage` "/Game/AI_DIOPORCO/Animations/HitReact_Front_Montage.HitReact_Front_Montage")
        (set `self.SaveAttack` false)
        (set `self.AttackCount` 0)
        (set `self.Attacking?` false)))
    (else
      (goto _label_4))))

(event `self.Box.OnComponentBeginOverlap`
  (params (OverlappedComponent :type "PrimitiveComponent Object Reference") (OtherActor :type "Actor Object Reference") (OtherComp :type "PrimitiveComponent Object Reference") (OtherBodyIndex :type Integer) (bFromSweep :type Boolean) (SweepResult :type "HitResult Structure (by ref)"))
  ;[1 1 1] Deal Damage
  (bind _asthird_person_character (cast `/Game/Cover_System/ThirdPersonCharacter` OtherActor))
  (if (`self.AttackRdy_0`)
    (`/Engine/EditorBlueprintResources/StandardMacros.DoOnce` false :!label _label_5
      (:`Completed`
        (`GameplayStatics.ApplyDamage` _asthird_person_character 10.0 null self)
        (`KismetSystemLibrary.Delay` 0.5)
        (goto _label_5 :!via `Reset`)))))

(event `/Game/AI_DIOPORCO/AttackBlockBP.Attack Blocked`
  ;[1 1 1] Enemy Blocked Attack
  (`self.PlayAnimMontage` "/Game/AI_DIOPORCO/Animations/Stun_Block/Stun_Short_Montage.Stun_Short_Montage")
  (set `self.SaveAttack` false)
  (set `self.AttackCount` 0)
  (set `self.Attacking?` false)
  (set `self.AttackRdy_0` false)
  (set `self.Stunned` true)
  (`KismetSystemLibrary.Delay` 1.0)
  (set `self.Stunned` false))

(fn `BlockAngleCheck`
  (returns (FaceinAI :type Boolean))
  (bind (_returnvalue_roll _returnvalue_pitch _returnvalue_yaw) (`KismetMathLibrary.BreakRotator` (`self.K2_GetActorRotation`)))
  (bind (_returnvalue_roll_2 _returnvalue_pitch_2 _returnvalue_yaw_2) (`KismetMathLibrary.BreakRotator` (`self.K2_GetActorRotation` (`self.AttackingActor`))))
  (bind _returnvalue (- _returnvalue_yaw _returnvalue_yaw_2))
  (return (or (> _returnvalue 150.0) (< _returnvalue -150.0))))

(fn `UserConstructionScript`)