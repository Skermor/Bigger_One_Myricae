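; BP_DreamSolvent is a projectile actor that is launched from whatever it is attached to, with a Niagara effect for its look.
; Shooting detaches it, sets movement velocity and facing from the given direction and speed, and switches the effect from summon to trail.
; After a short fixed delay it destroys itself by deactivating the effect and setting a brief lifespan so particles can fade.
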(event `Shoot_DreamSolvent`
  (params (Direction :type "Vector Structure") (Speed :type "Float (double-precision)"))
  (bind _dreamsolvent_fx (`self.DreamSolvent_FX`))
  (`self.K2_DetachFromActor` "KeepWorld" "KeepWorld" "KeepWorld")
  (set `MovementComponent.Velocity` (* Direction Speed) (`self.DreamSolventMovement`))
  (`self.K2_SetActorRotation` (`KismetMathLibrary.Conv_VectorToRotator` Direction))
  (`NiagaraComponent.SetVariableFloat` _dreamsolvent_fx "User.TrailRate" 1.0)
  (`NiagaraComponent.SetVariableFloat` _dreamsolvent_fx "User.SummonRate" 0.0)
  (`KismetSystemLibrary.Delay` 3.0)
  (`self.Destroy_DreamSolvent`))

(event `Destroy_DreamSolvent`
  (`ActorComponent.Deactivate` (`self.DreamSolvent_FX`))
  (`self.SetLifeSpan` 2.0))

(fn `UserConstructionScript`)